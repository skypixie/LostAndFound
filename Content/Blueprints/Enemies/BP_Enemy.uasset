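; BP_Enemy is a sprite-based enemy that chases a given pawn.
; On BeginPlay it randomizes its max walk speed and scales the sprite's play rate by a random factor, so instances vary in movement and animation.
; ChasePawn calls the parent implementation, then issues AI Move To toward that pawn, stopping on overlap.
; Tick forces a fixed actor rotation with physics teleport, keeping orientation constant while moving.
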(event `self.ReceiveBeginPlay`
  (bind _sprite (`self.Sprite`))
  (set `CharacterMovementComponent.MaxWalkSpeed` (`KismetMathLibrary.Conv_IntToDouble` (`KismetMathLibrary.RandomIntegerInRange` 200 700)) (`self.MovementPtr`))
  (`PaperFlipbookComponent.SetPlayRate` _sprite (* (`KismetMathLibrary.RandomFloatInRange` 0.7 1.4) (`PaperFlipbookComponent.GetPlayRate` _sprite))))

(event `self.ReceiveTick`
  (params (DeltaSeconds :type "Float (single-precision)"))
  (`self.K2_SetActorRotation` (struct :`Yaw` 180.0) true))

(event `self.ChasePawn`
  (params (Pawn :type "Pawn Object Reference"))
  (`parent.ChasePawn` Pawn)
  (`|AIMoveTo` self (0.0 0.0 0.0) Pawn 5.0 true))

(fn `UserConstructionScript`)