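; Boss enemy for a Paper2D-style game, with health, a delayed shockwave attack and timed hit reactions, its rotation locked every tick.
; Damage lowers health and blocks attacking through BP_AI_Boss until a short timer ends, or destroys the actor after that delay at zero health.
; Attack starts a timer that spawns BP_ShockImpact below the boss, calls the hero's hit handler without a range check and repositions the sprite.
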(event `self.ReceiveBeginPlay`
  (add `self.OnTakeAnyDamage` (delegate `OnTakeAnyDamage_Event`)))

(event `OnTakeAnyDamage_Event` :!signature `self.OnTakeAnyDamage`
  (params (DamagedActor :type "Actor Object Reference") (Damage :type "Float (single-precision)") (DamageType :type "DamageType Object Reference") (InstigatedBy :type "Controller Object Reference") (DamageCauser :type "Actor Object Reference"))
  (set `self.Health` (- (`self.Health`) Damage))
  (bind _asbp_ai_boss (cast `/Game/Blueprints/Enemies/Boss/BP_AI_Boss` (`self.GetController`)))
  (`/Game/Blueprints/Enemies/Boss/BP_AI_Boss.SetCanAttack` _asbp_ai_boss false)
  (set `self.bIsTakingDamage` true)
  (`KismetSystemLibrary.K2_SetTimer` null "ReceiveDamageEnd" 0.45)
  (if (<= (`self.Health`) 0.0)
    (`KismetSystemLibrary.K2_SetTimer` null "Die" 0.45)))

(event `self.ReceiveTick`
  (params (DeltaSeconds :type "Float (single-precision)"))
  (`self.K2_SetActorRotation` (struct :`Yaw` 180.0)))

(event `/Game/Blueprints/Enemies/Boss/BPI_BossFight.Attack`
  (`KismetSystemLibrary.K2_SetTimer` null "PlayAttackAnimEnd" 0.8))

(fn `Die`
  (`self.K2_DestroyActor`))

(fn `PlayAttackAnimEnd`
  (bind (_returnvalue_x _returnvalue_y _returnvalue_z) (`KismetMathLibrary.BreakVector` (`self.K2_GetActorLocation`)))
  (set `self.bIsAttacking` false)
  (`|SpawnActorFromClass` "/Game/Blueprints/WorldObjects/BP_ShockImpact.BP_ShockImpact_C" (`KismetMathLibrary.MakeTransform` (`KismetMathLibrary.MakeVector` _returnvalue_x _returnvalue_y (- _returnvalue_z 80.0))) "AlwaysSpawn" "MultiplyWithRoot" null null)
  (bind _asbp_paper_hero (cast `/Game/Blueprints/Character/BP_PaperHero` (`GameplayStatics.GetPlayerCharacter` 0)))
  (`/Game/Blueprints/Character/BP_PaperHero.GetHitByboss` _asbp_paper_hero self)
  (`SceneComponent.K2_SetRelativeLocation` (`self.Sprite`) (0.0 0.0 20.0) false false))

(fn `ReceiveDamageEnd`
  (set `self.bIsTakingDamage` false)
  (bind _asbp_ai_boss (cast `/Game/Blueprints/Enemies/Boss/BP_AI_Boss` (`self.GetController`)))
  (`/Game/Blueprints/Enemies/Boss/BP_AI_Boss.SetCanAttack` _asbp_ai_boss true))

(fn `UserConstructionScript`)