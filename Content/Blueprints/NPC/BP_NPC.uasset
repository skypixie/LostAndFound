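; BP_NPC is an NPC that the player hero can talk to, showing its dialogue lines one at a time.
; A collision overlap toggles the BP_PaperHero's CanTalk flag and its "Press E to Talk" hint.
; Each Talk call displays the next entry of Lines in a WBP_Talk widget, created if the stored UI reference is invalid.
; After the last line, it removes all WBP_Talk widgets and resets the line index.
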(event `self.DialogueCollision.OnComponentBeginOverlap`
  (params (OverlappedComponent :type "PrimitiveComponent Object Reference") (OtherActor :type "Actor Object Reference") (OtherComp :type "PrimitiveComponent Object Reference") (OtherBodyIndex :type Integer) (bFromSweep :type Boolean) (SweepResult :type "HitResult Structure (by ref)"))
  (bind _asbp_paper_hero (cast `/Game/Blueprints/Character/BP_PaperHero` OtherActor))
  (set `/Game/Blueprints/Character/BP_PaperHero.bCanTalk` true _asbp_paper_hero)
  (`/Game/Blueprints/Character/BP_PaperHero.SetHintText` _asbp_paper_hero "Press E to Talk"))

(event `self.DialogueCollision.OnComponentEndOverlap`
  (params (OverlappedComponent :type "PrimitiveComponent Object Reference") (OtherActor :type "Actor Object Reference") (OtherComp :type "PrimitiveComponent Object Reference") (OtherBodyIndex :type Integer))
  (bind _asbp_paper_hero (cast `/Game/Blueprints/Character/BP_PaperHero` OtherActor))
  (set `/Game/Blueprints/Character/BP_PaperHero.bCanTalk` false _asbp_paper_hero)
  (`/Game/Blueprints/Character/BP_PaperHero.SetHintText` _asbp_paper_hero ""))

(fn `Talk`
  (locals (UI :type "/Game/Blueprints/UI/WBP_Talk Object Reference"))
  (bind _lines (`self.Lines`))
  (bind _lineind (`self.LineInd`))
  (`local.UI`
    (:`then`
      _)
    (:`else`
      (bind _returnvalue (`|CreateWidget` "/Game/Blueprints/UI/WBP_Talk.WBP_Talk_C" (`GameplayStatics.GetPlayerController` 0)))
      (bind _output_get (set `local.UI` _returnvalue))
      (`UserWidget.AddToViewport` _output_get 0)))
  (if (< _lineind (`KismetArrayLibrary.Array_Length` _lines))
    (set `TextBlock.Text` (`KismetTextLibrary.Conv_StringToText` (`|GetArrayItem` _lines _lineind)) (`/Game/Blueprints/UI/WBP_Talk.TalkText` (`local.UI`)))
    (`/Engine/EditorBlueprintResources/StandardMacros.IncrementInt` (`self.LineInd`))
    (else
      (bind _foundwidgets (`WidgetBlueprintLibrary.GetAllWidgetsOfClass` "/Game/Blueprints/UI/WBP_Talk.WBP_Talk_C" false))
      (for _array_element _foundwidgets
        (`Widget.RemoveFromParent` _array_element))
      (set `self.LineInd` 0))))

(fn `UserConstructionScript`)